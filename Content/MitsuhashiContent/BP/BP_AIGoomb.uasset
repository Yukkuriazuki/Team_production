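; AI controller, apparently for a Goomba-style enemy, that keeps its pawn walking in a straight line along the X axis.
; From BeginPlay, Movement issues an AI move to a point MoveSpeed away from the pawn, then re-calls itself after a short delay without waiting for the move to finish.
; Lnversion negates MoveSpeed to reverse the walking direction; nothing in this Blueprint calls it.
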(event `self.ReceiveBeginPlay`
  (`self.Movement`))

(event `self.ReceiveTick`
  (params (DeltaSeconds :type "Float (single-precision)")))

(event `Movement`
  (bind _returnvalue (`self.K2_GetPawn`))
  (bind (_returnvalue_x _returnvalue_y _returnvalue_z) (`KismetMathLibrary.BreakVector` (`self.K2_GetActorLocation` _returnvalue)))
  (`|AIMoveTo` _returnvalue (`KismetMathLibrary.MakeVector` (+ _returnvalue_x (`self.MoveSpeed`)) _returnvalue_y _returnvalue_z) null
    (:`then`
      (`KismetSystemLibrary.Delay` 0.2)
      (`self.Movement`))))

(fn `Lnversion`
  (set `self.MoveSpeed` (* -1 (`self.MoveSpeed`))))

(fn `UserConstructionScript`)