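; Game mode that runs a match countdown and respawns the player whenever their pawn is destroyed.
; On BeginPlay it starts a looping one-second timer and binds to player 0 pawn's OnDestroyed event.
; Destruction calls RestartPlayer, then rebinds to the new pawn so respawning keeps working.
; Each tick of the timer decrements TimeLeft; once it runs out, the destroy bindings are cleared and the End level opens.
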(event `self.ReceiveBeginPlay`
  (`self.Time`)
  (`self.RestartEvent`))

(event `RestartEvent`
  (add `self.OnDestroyed` (`GameplayStatics.GetPlayerPawn` 0) (delegate `RestartThirdPerson`)))

(event `RestartThirdPerson` :!signature `self.OnDestroyed`
  (params (DestroyedActor :type "Actor Object Reference"))
  (`self.RestartPlayer` (`GameplayStatics.GetPlayerController` 0))
  (`self.RestartEvent`))

(event `Time`
  (`KismetSystemLibrary.K2_SetTimerDelegate` (delegate `CountDown`) 1.0 true))

(event `CountDown`
  (bind _timeleft (`self.TimeLeft`))
  (if (> (`KismetMathLibrary.Conv_IntToByte` _timeleft) 0)
    (set `self.TimeLeft` (- _timeleft 1))
    (else
      (clear `self.OnDestroyed` (`GameplayStatics.GetPlayerPawn` 0))
      (`GameplayStatics.OpenLevel` "End"))))

(fn `UserConstructionScript`)